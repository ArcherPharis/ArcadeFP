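; Whack-a-mole "good" target actor that pops up when spawned and retracts when despawned.
; On BeginPlay a timeline lerps it upward from its spawn location by a fixed height.
; Despawn reverses that timeline, disables mesh collision and clears the occupancy flag on its owning BP_WAMTargetSpawner.
; Hit handling, scoring and actor destruction are not part of this graph.
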(event `self.ReceiveBeginPlay`
  (bind _output_get (set `self.start` (`self.K2_GetActorLocation`)))
  (bind _output_get_2 (set `self.end` (+ _output_get (0.0 0.0 420.0))))
  (bind (_direction _alpha) (`Timeline|Timeline_0` :!label _label)
    (:`Update`
      (`self.K2_SetActorLocation` (`KismetMathLibrary.VLerp` _output_get _output_get_2 _alpha)))))

(event `self.Despawn`
  (`|ExecutionSequence`
    (:`then_0`
      (goto _label :!via `ReverseFromEnd`))
    (:`then_1`
      (`PrimitiveComponent.SetCollisionEnabled` (`self.GetMesh`) "NoCollision"))
    (:`then_2`
      (bind _asbp_wamtarget_spawner (cast `/Game/Blueprint/ArcadeStations/WhackAMole/Targets/BP_WAMTargetSpawner` (`self.GetOwner`)))
      (`WAMTargetSpawner.SetOccupancy` _asbp_wamtarget_spawner false))))

(fn `UserConstructionScript`)