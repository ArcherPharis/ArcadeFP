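; Enemy card player actor for the arcade card game that animates cards the opponent plays.
; MoveCard lerps a card by timeline from the actor's location to PlayedCards, attaches it there, then replaces and destroys the previous card.
; ClearDeck waits briefly, slides the last played card to ClearDeckDestination, then calls HandleTieSkirmish on the card game mode.
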(event `self.MoveCard`
  (params (cardToMove :type "BaseCard Object Reference"))
  (bind _previouscard (`self.PreviousCard`))
  (set `self.start` (`self.K2_GetActorLocation`))
  (set `self.end` (`SceneComponent.K2_GetComponentLocation` (`self.PlayedCards`)))
  (bind (_direction _alpha) (`Timeline|Timeline_0` :!via `PlayFromStart`)
    (:`Update`
      (`self.K2_SetActorLocation` cardToMove (`KismetMathLibrary.VLerp` (`self.start`) (`self.end`) _alpha) false false)
      (`self.K2_AttachToComponent` cardToMove (`self.PlayedCards`) "None" "KeepRelative" "KeepRelative" "KeepRelative" true))
    (:`Finished`
      (`/Engine/EditorBlueprintResources/StandardMacros.IsValid` _previouscard
        (:`Is Valid`
          (`self.K2_DestroyActor` _previouscard)
          (set `self.PreviousCard` cardToMove))
        (:`Is Not Valid`
          (set `self.PreviousCard` cardToMove))))))

(event `self.ClearDeck`
  (`KismetSystemLibrary.Delay` 2.7)
  (`/Engine/EditorBlueprintResources/StandardMacros.IsValid` (`self.PreviousCard`)
    (:`Is Valid`
      (set `self.deckStart` (`self.K2_GetActorLocation` (`self.PreviousCard`)))
      (bind (_direction _alpha) (`Timeline|Timeline_1` :!via `PlayFromStart`)
        (:`Update`
          (`self.K2_SetActorLocation` (`self.PreviousCard`) (`KismetMathLibrary.VLerp` (`self.deckStart`) (`SceneComponent.K2_GetComponentLocation` (`self.ClearDeckDestination`)) _alpha) false false))
        (:`Finished`
          (`CardGameMode.HandleTieSkirmish` (`self.GetCardGameMode`)))))
    (:`Is Not Valid`
      (`KismetSystemLibrary.PrintString` "Hello"))))

(fn `UserConstructionScript`)