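; Actor for the arcade card game that moves a played card onto the played-cards spot.
; MoveCard runs a timeline that lerps the given card from its current location to the PlayedCards component's world location.
; When the move finishes, it destroys the previously played card, if valid, and stores the new one as PreviousCard, leaving only the latest card in place.
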(event `self.MoveCard`
  (params (cardToMove :type "BaseCard Object Reference"))
  (bind _previouscard (`self.PreviousCard`))
  (set `self.start` (`self.K2_GetActorLocation` cardToMove))
  (set `self.end` (`SceneComponent.K2_GetComponentLocation` (`self.PlayedCards`)))
  (bind (_direction _alpha) (`Timeline|MoveTheCard` :!via `PlayFromStart`)
    (:`Update`
      (`self.K2_SetActorLocation` cardToMove (`KismetMathLibrary.VLerp` (`self.start`) (`self.end`) _alpha) false false))
    (:`Finished`
      (`/Engine/EditorBlueprintResources/StandardMacros.IsValid` _previouscard
        (:`Is Valid`
          (`self.K2_DestroyActor` _previouscard)
          (set `self.PreviousCard` cardToMove))
        (:`Is Not Valid`
          (set `self.PreviousCard` cardToMove))))))

(fn `UserConstructionScript`)